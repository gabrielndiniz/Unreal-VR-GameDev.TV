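; Hand controller actor that detects when the hand can climb by overlapping actors tagged Climbable.
; Every begin overlap passes a can-climb flag based only on the new actor's tag, then adds climbable actors to an Overlapping list.
; End overlaps of climbable actors remove them from the list and pass whether any remain.
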(event Collision|EventActorBeginOverlap
  (params (OtherActor :type Actor%20Object%20Reference))
  (bind _returnvalue (Actor|ActorHasTag OtherActor "Climbable"))
  (Class|HandController|ActorBeginOverlap self OtherActor _returnvalue)
  (if _returnvalue
    (Utilities|Array|Add (Variables|Default|GetOverlapping) OtherActor)))

(event Collision|EventActorEndOverlap
  (params (OtherActor :type Actor%20Object%20Reference))
  (bind _overlapping (Variables|Default|GetOverlapping))
  (if (Actor|ActorHasTag OtherActor "Climbable")
    (Utilities|Array|RemoveItem _overlapping OtherActor)
    (Class|HandController|ActorEndOverlap self OtherActor (Utilities|Array|IsValidIndex _overlapping))))

(fn ConstructionScript)